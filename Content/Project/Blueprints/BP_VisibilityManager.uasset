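; BP_VisibilityManager is a manager actor that shows or hides tagged groups of actors in game.
; On BeginPlay it enables the mouse cursor with Game and UI input, creates WBP_VisibilityManager with a self reference, and applies each TagsArray entry's StartVisible.
; SetVisibilityOnTag toggles one tag's actors, but its ForAll branch sets only the manager's own visibility from StartVisible.
; SetVisibilityForAll is an empty stub.
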(event `self.ReceiveBeginPlay`
  (bind _returnvalue (`GameplayStatics.GetPlayerController` 0))
  (`WidgetBlueprintLibrary.SetInputMode_GameAndUIEx` _returnvalue null)
  (set `PlayerController.bShowMouseCursor` true _returnvalue)
  (bind _returnvalue_2 (`|CreateWidget` "/Game/Project/Blueprints/Widgets/WBP_VisibilityManager.WBP_VisibilityManager_C" null self))
  (bind _output_get (set `self.WBP_VisibilityManager` _returnvalue_2))
  (`UserWidget.AddToViewport` _output_get 0)
  (for _array_element (`self.TagsArray`)
    (bind (_name _tag _bstartvisible) (break `/Game/Project/S_Tag` _array_element))
    (bind _outactors (`GameplayStatics.GetAllActorsWithTag` _tag))
    (for _array_element_2 _outactors
      (`self.SetActorHiddenInGame` _array_element_2 (not _bstartvisible)))))

(event `Set Visibility On Tag`
  (params (bForAll :type Boolean) (Tag :type Name) (bIsVisible :type Boolean))
  (if bForAll
    (for _array_element (`self.TagsArray`)
      (bind (_name _tag _bstartvisible) (break `/Game/Project/S_Tag` _array_element))
      (bind _outactors (`GameplayStatics.GetAllActorsWithTag` _tag))
      (for _ _outactors
        (`self.SetActorHiddenInGame` (not _bstartvisible))))
    (else
      (bind _outactors_2 (`GameplayStatics.GetAllActorsWithTag` Tag))
      (for _array_element_2 _outactors_2
        (`self.SetActorHiddenInGame` _array_element_2 (not bIsVisible))))))

(event `Set Visibility For All`
  (params (bIsVisible :type Boolean)))

(fn `UserConstructionScript`)