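; BP_VisManager is a manager Blueprint that shows or hides groups of level actors by actor tag.
; On BeginPlay it enables Game-and-UI input with the cursor, adds a WBP_VisibilityManager widget to the viewport, and applies each TagsArray entry's initial visibility.
; SetVisOnTag and SetVisForAll change visibility for one tag or all listed tags.
; Only each tagged actor's root component is toggled, without propagating to children.
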(event `Set Vis On Tag`
  (params (Tag :type Name) (bIsVisible :type Boolean))
  (bind _outactors (`GameplayStatics.GetAllActorsWithTag` Tag))
  (for _array_element _outactors
    (`SceneComponent.SetVisibility` (`Actor.RootComponent` _array_element) bIsVisible false)))

(event `Set Vis For All`
  (params (bIsVisible :type Boolean))
  (for _array_element (`self.TagsArray`)
    (bind _outactors (`GameplayStatics.GetAllActorsWithTag` (`.Tag_6_3ACE90B0416CF2A0191008A358107F66` (break `/Game/Project/S_tags` _array_element))))
    (for _array_element_2 _outactors
      (`SceneComponent.SetVisibility` (`Actor.RootComponent` _array_element_2) bIsVisible false))))

(event `self.ReceiveBeginPlay`
  (bind _returnvalue (`GameplayStatics.GetPlayerController` 0))
  (`WidgetBlueprintLibrary.SetInputMode_GameAndUIEx` _returnvalue null)
  (set `PlayerController.bShowMouseCursor` true _returnvalue)
  (bind _returnvalue_2 (`|CreateWidget` "/Game/Project/Blueprints/Widgets/WBP_VisibilityManager.WBP_VisibilityManager_C"))
  (bind _output_get (set `self.WBP_VisibilityManager` _returnvalue_2))
  (`UserWidget.AddToViewport` _output_get 0)
  (for _array_element (`self.TagsArray`)
    (bind (_name _tag _bisvisible) (break `/Game/Project/S_tags` _array_element))
    (bind _outactors (`GameplayStatics.GetAllActorsWithTag` _tag))
    (for _array_element_2 _outactors
      (`SceneComponent.SetVisibility` (`Actor.RootComponent` _array_element_2) _bisvisible false))))

(fn `UserConstructionScript`)